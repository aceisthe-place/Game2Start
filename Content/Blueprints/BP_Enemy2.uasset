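; BP_Enemy2 is a simple enemy Blueprint that tracks Health and destroys itself when that runs out.
; On BeginPlay it prints an Inigo Montoya quote.
; Its TakeDamage event prints a pain message, subtracts the incoming amount from Health, then uses the CheckIfDead function to decide whether to destroy the actor.
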(event `self.ReceiveBeginPlay`
  (`KismetSystemLibrary.PrintString` "My name is Inigo Montoya. You killed my father. Prepare to die."))

(event `TakeDamage`
  (params (ByAmount :type "Float (double-precision)" :default 0.2))
  (`KismetSystemLibrary.PrintString` "Yeeeeeeouch!!!!")
  (set `self.Health` (- (`self.Health`) ByAmount))
  (if (`self.CheckIfDead` (`self.Health`))
    (`self.K2_DestroyActor`)))

(fn `CheckIfDead`
  (params (Health :type "Float (double-precision)"))
  (returns (IsDead :type Boolean))
  (return (<= Health 0.0)))

(fn `UserConstructionScript`)