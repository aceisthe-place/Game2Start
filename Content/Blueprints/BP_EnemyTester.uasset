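; BP_EnemyTester is a test Blueprint that repeatedly damages every BP_Enemy2 actor in the level.
; From BeginPlay it finds all enemies with GetAllActorsOfClass, prints their count, and calls TakeDamage on each with a small random amount.
; It then prints a confirmation, waits on a Delay, and calls its own GiveDamage event, so the cycle repeats indefinitely with a fresh enemy search each pass.
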(event `GiveDamage`
  (bind _outactors (`GameplayStatics.GetAllActorsOfClass` "/Game/Blueprints/BP_Enemy2.BP_Enemy2_C" :!label _label)) ; Find all BP_Enemies
  (`KismetSystemLibrary.PrintString` (`KismetStringLibrary.Concat_StrStr` "there are " (`KismetStringLibrary.Conv_IntToString` (`KismetArrayLibrary.Array_Length` _outactors)) " enemies"))
  (for _array_element _outactors
    (`/Game/Blueprints/BP_Enemy2.TakeDamage` _array_element (`KismetMathLibrary.RandomFloatInRange` 0.1 0.5)))
  (`KismetSystemLibrary.PrintString` "We've given damage to all enemies")
  (`KismetSystemLibrary.Delay` 2.0)
  (`self.GiveDamage`))

(event `self.ReceiveBeginPlay`
  (goto _label))

(fn `UserConstructionScript`)